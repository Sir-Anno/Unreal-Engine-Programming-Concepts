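; BP_SimpleDoor is a networked door that swings open when a character enters its collision box and closes when an overlap ends.
; The server compares door and character forward vectors to pick a 90-degree swing direction, then sets IsOpen.
; The IsOpen RepNotify plays or reverses the OpenClose timeline, which lerps the Pivot's relative rotation toward the chosen angle.
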(event OnComponentBeginOverlap(CollisionBox)
  (params (OverlappedComponent :type Primitive%20Component%20Object%20Reference) (OtherActor :type Actor%20Object%20Reference) (OtherComp :type Primitive%20Component%20Object%20Reference) (OtherBodyIndex :type Integer) (bFromSweep :type Boolean) (SweepResult :type Hit%20Result%20Structure%20%28by%20ref%29))
  (Networking|SwitchHasAuthority ; Only run on server
    (:Authority
      (bind _ascharacter (Utilities|Casting|CastToCharacter OtherActor))
      (if (Utilities|Operators|EqualEqual (Transformation|GetActorForwardVector) (Math|Vector|GetForwardVector (Variables|/Script/Engine.Actor|GetRootComponent _ascharacter)) 0.5)
        (Variables|Default|SetRotationAngle "0.000000,-90.000000,0.000000")
        (else
          (Variables|Default|SetRotationAngle "0.000000,90.000000,0.000000")))
      (Variables|Default|SetIsOpen true))))

(event OnComponentEndOverlap(CollisionBox)
  (params (OverlappedComponent :type Primitive%20Component%20Object%20Reference) (OtherActor :type Actor%20Object%20Reference) (OtherComp :type Primitive%20Component%20Object%20Reference) (OtherBodyIndex :type Integer))
  (Variables|Default|SetIsOpen false))

(event Custom|OpenDoor
  (bind _alpha (Timeline|Open%20/%20Close Play)
    (:Update
      (Transformation|SetRelativeRotation (Variables|Default|GetPivot) (Math|Rotator|Lerp(Rotator) "0, 0, 0" (Variables|Default|GetRotationAngle) _alpha true) false false))))

(event Custom|CloseDoor
  (bind _alpha (Timeline|Open%20/%20Close Reverse)
    (:Update
      (Transformation|SetRelativeRotation (Variables|Default|GetPivot) (Math|Rotator|Lerp(Rotator) "0, 0, 0" (Variables|Default|GetRotationAngle) _alpha true) false false))))

(fn ConstructionScript)

(fn OnRepIsOpen
  (if (Variables|Default|GetIsOpen)
    (CallFunction|OpenDoor)
    (else
      (CallFunction|CloseDoor))))