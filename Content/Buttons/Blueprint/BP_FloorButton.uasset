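; A floor button that sinks when something overlaps its sphere collision and activates linked actors.
; Overlap begin and end are handled only with authority, calling Trigger and Reset.
; Trigger plays a click sound and runs a timeline that lowers the mesh, while Reset reverses it.
; Only a completed forward press sends InteractMessage to each actor in ActorsToTrigger; release sends nothing.
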(event OnComponentBeginOverlap(SphereCollision)
  (params (OverlappedComponent :type Primitive%20Component%20Object%20Reference) (OtherActor :type Actor%20Object%20Reference) (OtherComp :type Primitive%20Component%20Object%20Reference) (OtherBodyIndex :type Integer) (bFromSweep :type Boolean) (SweepResult :type Hit%20Result%20Structure%20%28by%20ref%29))
  (Networking|SwitchHasAuthority
    (:Authority
      (CallFunction|Trigger))))

(event OnComponentEndOverlap(SphereCollision)
  (params (OverlappedComponent :type Primitive%20Component%20Object%20Reference) (OtherActor :type Actor%20Object%20Reference) (OtherComp :type Primitive%20Component%20Object%20Reference) (OtherBodyIndex :type Integer))
  (Networking|SwitchHasAuthority
    (:Authority
      (CallFunction|Reset))))

(event Custom|Trigger
  (Audio|PlaySoundatLocation "/Engine/VREditor/Sounds/UI/Click_on_Button_Cue.Click_on_Button_Cue" (Transformation|GetActorLocation) "0, 0, 0" 1.0 1.0 0.0 0 0 0 0)
  (bind (_direction _push_button) (Timeline|Push%20Button Play)
    (:Update
      (Transformation|SetRelativeLocation (Variables|Default|GetButtonMesh) (Math|Vector|Lerp(Vector) "0, 0, 0" "0.000000,0.000000,-5.000000" _push_button) false false))
    (:Finished
      (switch Utilities|FlowControl|Switch|SwitchonETimelineDirection _direction
        (:Forward
          (for _array_element (Variables|Default|GetActorsToTrigger)
            (Class|BPInteractInterface|Interact(Message) _array_element)))))))

(event Custom|Reset
  (bind (_direction _push_button) (Timeline|Push%20Button Reverse)
    (:Update
      (Transformation|SetRelativeLocation (Variables|Default|GetButtonMesh) (Math|Vector|Lerp(Vector) "0, 0, 0" "0.000000,0.000000,-5.000000" _push_button) false false))
    (:Finished
      (switch Utilities|FlowControl|Switch|SwitchonETimelineDirection _direction
        (:Forward
          (for _array_element (Variables|Default|GetActorsToTrigger)
            (Class|BPInteractInterface|Interact(Message) _array_element)))))))

(fn ConstructionScript)