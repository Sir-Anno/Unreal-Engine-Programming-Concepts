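; BP_PushButton is an interactable push button that sends TriggerMessage to every actor in its ActorsToTrigger list.
; Interact fires Trigger only with authority, and a DoOnce blocks repeat presses while a click sound plays and a timeline lowers the button mesh.
; When the timeline finishes, each listed actor is messaged and Reset re-arms the DoOnce inside that loop, so an empty list leaves the button locked.
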(event Custom|Reset
  (Utilities|FlowControl|DoOnce false) ; enters at Reset
)

(event Custom|Trigger
  (Utilities|FlowControl|DoOnce false
    (:Completed
      (Audio|PlaySoundatLocation "/Engine/VREditor/Sounds/UI/Click_on_Button_Cue.Click_on_Button_Cue" (Transformation|GetActorLocation) "0, 0, 0" 1.0 1.0 0.0 0 0 0 0)
      (bind _push_button (Timeline|Push%20Button PlayFromStart)
        (:Update
          (Transformation|SetRelativeLocation (Variables|Default|GetButtonMesh) (Math|Vector|Lerp(Vector) "0, 0, 0" "0.000000,0.000000,-5.000000" _push_button) false false))
        (:Finished
          (for _array_element (Variables|Default|GetActorsToTrigger)
            (Class|BPTriggerInterface|Trigger(Message) _array_element)
            (CallFunction|Reset)))))))

(event EventInteract
  (Networking|SwitchHasAuthority
    (:Authority
      (CallFunction|Trigger))))

(fn ConstructionScript)