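; BP_ColorCube is an interactable cube that changes to a random color when used.
; BeginPlay creates a dynamic instance of M_ColorCube on its static mesh.
; Interact acts only on authority, setting Color to a random fully saturated, full-brightness hue.
; The Color RepNotify writes the value to the material's Color parameter, keeping the look in sync across the network.
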(event Custom|Set%20color
  (Variables|Default|SetColor (CallFunction|GetRandomColor)))

(event EventInteract
  (Networking|SwitchHasAuthority
    (:Authority
      (CallFunction|SetColor))))

(event EventBeginPlay
  (bind _returnvalue (Rendering|Material|CreateDynamicMaterialInstance (Variables|Default|GetStatic%20mesh) 0 "/Game/Interactables/ColorCube/M_ColorCube.M_ColorCube" "None" :!class /Script/Engine.PrimitiveComponent))
  (Variables|Default|SetMaterialInstance _returnvalue))

(fn ConstructionScript)

(fn OnRepColor
  (Rendering|Material|SetVectorParameterValue (Variables|Default|GetMaterialInstance) "Color" (Variables|Default|GetColor) :!class /Script/Engine.MaterialInstanceDynamic))

(fn GetRandomColor
  (return (Class|KismetMathLibrary|HSVtoRGB (Math|Random|RandomFloatinRange 0.0 359.0) 1.0 1.0 1.0)))